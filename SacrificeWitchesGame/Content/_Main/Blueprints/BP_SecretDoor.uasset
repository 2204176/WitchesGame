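; Secret bookcase door that the player triggers with E while standing inside a box trigger, which enables input and opens a gate.
; A FlipFlop alternates between a timeline that tilts the special book and swings the bookcase, and a second reversed timeline.
; The second timeline only holds the bookcase yaw at zero, leaving the book untouched.
; A separate sphere trigger shows and hides a widget.
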(event OnComponentBeginOverlap(Sphere)
  (params (OverlappedComponent :type Primitive%20Component%20Object%20Reference) (OtherActor :type Actor%20Object%20Reference) (OtherComp :type Primitive%20Component%20Object%20Reference) (OtherBodyIndex :type Integer) (bFromSweep :type Boolean) (SweepResult :type Hit%20Result%20Structure%20%28by%20ref%29))
  (Rendering|SetVisibility (Variables|Default|GetWidget) true false))

(event OnComponentEndOverlap(Sphere)
  (params (OverlappedComponent :type Primitive%20Component%20Object%20Reference) (OtherActor :type Actor%20Object%20Reference) (OtherComp :type Primitive%20Component%20Object%20Reference) (OtherBodyIndex :type Integer))
  (Rendering|SetVisibility (Variables|Default|GetWidget) false false))

(event OnComponentBeginOverlap(Box)
  (params (OverlappedComponent :type Primitive%20Component%20Object%20Reference) (OtherActor :type Actor%20Object%20Reference) (OtherComp :type Primitive%20Component%20Object%20Reference) (OtherBodyIndex :type Integer) (bFromSweep :type Boolean) (SweepResult :type Hit%20Result%20Structure%20%28by%20ref%29))
  (Utilities|Casting|CastToBP_ThirdPersonCharacter OtherActor)
  (Input|EnableInput (Game|GetPlayerController 0))
  (Utilities|FlowControl|Gate true) ; enters at Open
)

(event OnComponentEndOverlap(Box)
  (params (OverlappedComponent :type Primitive%20Component%20Object%20Reference) (OtherActor :type Actor%20Object%20Reference) (OtherComp :type Primitive%20Component%20Object%20Reference) (OtherBodyIndex :type Integer))
  (Utilities|Casting|CastToBP_ThirdPersonCharacter OtherActor)
  (Input|DisableInput (Game|GetPlayerController 0))
  (Utilities|FlowControl|Gate true) ; enters at Close
)

(event EventBeginPlay)

(event Collision|EventActorBeginOverlap
  (params (OtherActor :type Actor%20Object%20Reference)))

(event EventTick
  (params (DeltaSeconds :type Float%20%28single-precision%29)))

(event Input|KeyboardEvents|E
  (params (Key :type Key%20Structure :default "None"))
  (:Pressed
    (if true
      (Utilities|FlowControl|Gate true
        (:Exit
          (Utilities|FlowControl|FlipFlop
            (:A
              (bind (_direction _booktrack _doortrack) (Timeline|OpenTRack Play)
                (:Update
                  (Transformation|SetRelativeRotation (Variables|Default|GetSpecialBook) (Math|Rotator|MakeRotator (Math|Float|Lerp (Variables|Default|GetBookIn) (Variables|Default|GetBookOut) _booktrack) 0.0 0.0) false false)
                  (Transformation|SetRelativeRotation (Variables|Default|GetBookCase) (Math|Rotator|MakeRotator 0.0 0.0 (Math|Float|Lerp (Variables|Default|GetDoorIn) (Variables|Default|GetDoorOut) _doortrack)) false false))))
            (:B
              (bind _door_track (Timeline|Timeline ReverseFromEnd)
                (:Update
                  (Transformation|SetRelativeRotation (Variables|Default|GetBookCase) (Math|Rotator|MakeRotator 0.0 0.0 (Math|Float|Lerp 0.0 0.0 _door_track)) false false))))))))))

(fn ConstructionScript)
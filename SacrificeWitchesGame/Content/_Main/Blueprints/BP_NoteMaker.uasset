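; BP_NoteMaker is a collectible book that shows a note card and sends the player to the Cave level when collected.
; Overlap enables its input and copies its NoteCardIndex to BP_ThirdPersonCharacter; ending overlap disables input.
; E toggles the NoteCardDisplay widget through a FlipFlop.
; C passes a gate opened by character overlap with the Box, then destroys the book and loads Cave after a short delay.
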(event OnComponentBeginOverlap(Box)
  (params (OverlappedComponent :type Primitive%20Component%20Object%20Reference) (OtherActor :type Actor%20Object%20Reference) (OtherComp :type Primitive%20Component%20Object%20Reference) (OtherBodyIndex :type Integer) (bFromSweep :type Boolean) (SweepResult :type Hit%20Result%20Structure%20%28by%20ref%29))
  ;[0 0 0] Collect Book and Travel to Next Level
  (Utilities|Casting|CastToBP_ThirdPersonCharacter OtherActor)
  (Input|EnableInput (Game|GetPlayerController 0))
  (Utilities|FlowControl|Gate true) ; enters at Open
)

(event Collision|EventActorBeginOverlap
  (params (OtherActor :type Actor%20Object%20Reference))
  ;[0 0 0] Add Multiple Images to Widget
  (Input|EnableInput (Game|GetPlayerController 0))
  (bind _asbp_third_person_character (Utilities|Casting|CastToBP_ThirdPersonCharacter (Game|GetPlayerCharacter 0)))
  (Variables|/Game/ThirdPerson/Blueprints/BP_ThirdPersonCharacter.BP_ThirdPersonCharacter_C|SetNoteCardIndex _asbp_third_person_character (Variables|Default|GetNote%20Card%20Index)))

(event Collision|EventActorEndOverlap
  (params (OtherActor :type Actor%20Object%20Reference))
  ;[0 0 0] Add Multiple Images to Widget
  (Input|DisableInput (Game|GetPlayerController 0)))

(event Input|KeyboardEvents|E
  (params (Key :type Key%20Structure :default "None"))
  ;[0 0 0] Open The Book
  (:Pressed
    (Utilities|FlowControl|FlipFlop
      (:A
        (bind _returnvalue (UserInterface|CreateWidget "/Game/_Main/Blueprints/NoteCardDisplay.NoteCardDisplay_C"))
        (UserInterface|Viewport|AddtoViewport _returnvalue 0))
      (:B
        (Widget|RemovefromParent _returnvalue)))))

(event Input|KeyboardEvents|C
  (params (Key :type Key%20Structure :default "None"))
  ;[0 0 0] Collect Book and Travel to Next Level
  (:Pressed
    (if true
      (Utilities|FlowControl|Gate true
        (:Exit
          (Utilities|FlowControl|Delay 0.5)
          (Actor|DestroyActor)
          (Game|OpenLevel(byObjectReference) "/Game/_Main/CaveLevel/Cave.Cave"))))))

(fn ConstructionScript)
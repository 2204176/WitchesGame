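; BP_OpenCell is a cell door that the player opens and closes with E, provided their character has a key.
; A trigger box detects BP_ThirdPersonCharacter, enabling input and opening a Gate on entry, then reversing both on exit.
; Pressing E checks HasKey and passes through the Gate to a FlipFlop, which plays or reverses a timeline that lerps the door's yaw between closed and open angles.
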(event OnComponentBeginOverlap(Box)
  (params (OverlappedComponent :type Primitive%20Component%20Object%20Reference) (OtherActor :type Actor%20Object%20Reference) (OtherComp :type Primitive%20Component%20Object%20Reference) (OtherBodyIndex :type Integer) (bFromSweep :type Boolean) (SweepResult :type Hit%20Result%20Structure%20%28by%20ref%29))
  (bind _asbp_third_person_character (Utilities|Casting|CastToBP_ThirdPersonCharacter OtherActor))
  (Input|EnableInput (Game|GetPlayerController 0))
  (Utilities|FlowControl|Gate true) ; enters at Open
)

(event OnComponentEndOverlap(Box)
  (params (OverlappedComponent :type Primitive%20Component%20Object%20Reference) (OtherActor :type Actor%20Object%20Reference) (OtherComp :type Primitive%20Component%20Object%20Reference) (OtherBodyIndex :type Integer))
  (Utilities|Casting|CastToBP_ThirdPersonCharacter OtherActor)
  (Input|DisableInput (Game|GetPlayerController 0))
  (Utilities|FlowControl|Gate true) ; enters at Close
)

(event Input|KeyboardEvents|E
  (params (Key :type Key%20Structure :default "None"))
  (:Pressed
    (if (Variables|/Game/ThirdPerson/Blueprints/BP_ThirdPersonCharacter.BP_ThirdPersonCharacter_C|GetHasKey? (stale OnComponentBeginOverlap(Box) _asbp_third_person_character))
      (Utilities|FlowControl|Gate true
        (:Exit
          (Utilities|FlowControl|FlipFlop
            (:A
              (bind _open_close_door (Timeline|Open/Vlose%20Door Play)
                (:Update
                  (Transformation|SetRelativeRotation (Variables|Default|GetDoor) (Math|Rotator|MakeRotator 0.0 0.0 (Math|Float|Lerp (Variables|Default|GetClosedAngle) (Variables|Default|GetOpen%20Angle) _open_close_door)) false false))))
            (:B
              (Timeline|Open/Vlose%20Door Reverse))))))))

(fn ConstructionScript)
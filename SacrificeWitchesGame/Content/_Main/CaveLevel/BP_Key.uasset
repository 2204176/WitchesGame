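; BP_Key is a collectible key in the cave level that starts hidden and appears with a sound after a fixed delay from BeginPlay.
; Overlapping its Box with BP_ThirdPersonCharacter enables input and opens a Gate, and leaving reverses both.
; Pressing E while the gate is open sets HasKey on the character and destroys the key.
; The Box overlap is active even while the key mesh is still hidden.
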(event OnComponentBeginOverlap(Box)
  (params (OverlappedComponent :type Primitive%20Component%20Object%20Reference) (OtherActor :type Actor%20Object%20Reference) (OtherComp :type Primitive%20Component%20Object%20Reference) (OtherBodyIndex :type Integer) (bFromSweep :type Boolean) (SweepResult :type Hit%20Result%20Structure%20%28by%20ref%29))
  (bind _asbp_third_person_character (Utilities|Casting|CastToBP_ThirdPersonCharacter OtherActor))
  (Input|EnableInput (Game|GetPlayerController 0))
  (Utilities|FlowControl|Gate true) ; enters at Open
)

(event OnComponentEndOverlap(Box)
  (params (OverlappedComponent :type Primitive%20Component%20Object%20Reference) (OtherActor :type Actor%20Object%20Reference) (OtherComp :type Primitive%20Component%20Object%20Reference) (OtherBodyIndex :type Integer))
  (Utilities|Casting|CastToBP_ThirdPersonCharacter OtherActor)
  (Input|DisableInput (Game|GetPlayerController 0))
  (Utilities|FlowControl|Gate true) ; enters at Close
)

(event Collision|EventActorBeginOverlap
  (params (OtherActor :type Actor%20Object%20Reference)))

(event EventTick
  (params (DeltaSeconds :type Float%20%28single-precision%29)))

(event EventBeginPlay
  (Rendering|SetVisibility (Variables|Default|GetKey) false true)
  (Utilities|FlowControl|Delay 5e+01)
  (Audio|PlaySound2D 0 1.0 1.0 0.0 0 0)
  (Rendering|SetVisibility (Variables|Default|GetKey) true true))

(event Input|KeyboardEvents|E
  (params (Key :type Key%20Structure :default "None"))
  (:Pressed
    (Utilities|FlowControl|Gate true
      (:Exit
        (Variables|/Game/ThirdPerson/Blueprints/BP_ThirdPersonCharacter.BP_ThirdPersonCharacter_C|SetHasKey? (stale OnComponentBeginOverlap(Box) _asbp_third_person_character) true)
        (Actor|DestroyActor)))))

(fn ConstructionScript)